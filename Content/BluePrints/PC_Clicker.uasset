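; Player controller for a clicker game that owns the UI and spawns enemies, items, floating damage-style text and cursor hit effects.
; On BeginPlay it caches the player pawn, shows the main widget, sets a custom cursor, and fills the level list and shop.
; Shop cards are built from DT_ItemInfo rows, then colored and enabled by comparing item cost to the pawn's coins.
; Main and ascension widgets are created lazily on show.
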(event Custom|SpawnEnemy
  (params (Enemy :type Actor%20Class%20Reference) (SpawnTransform :type Transform))
  ;[0.15 0.04255 0.1265 0.5] Spawn Enemy
  (bind _returnvalue (Game|SpawnActorfromClass Enemy SpawnTransform "AdjustIfPossibleButAlwaysSpawn" "MultiplyWithRoot" 0 0))
  (bind _enemy (Class|BPIEnemyBase|GetEnemyReference(Message) _returnvalue))
  (Variables|Default|SetSpawnedEnemy _enemy))

(event Custom|SpawnHitEffect
  ;[0.0624 0.1371 0.15 0.5] SpawnHitEffect
  (Game|SpawnActorfromClass "/Game/BluePrints/BP_HitEffect.BP_HitEffect_C" (Math|Conversions|ToTransform(Vector) (- (.WorldLocation (Game|Player|ConvertMouseLocationToWorldSpace)) "0.000000,1.000000,0.000000")) "AlwaysSpawn" "MultiplyWithRoot" 0 0))

(event Custom|SpawnFloatingText
  (params (SpawnLocation :type Vector) (Text :type String))
  (bind (_x _y _z) (Math|Vector|BreakVector SpawnLocation))
  ;[0.04998 0.15 0.1206 0.5] SpawnFloatingText
  (Game|SpawnActorfromClass "/Game/BluePrints/BP_FloatingText.BP_FloatingText_C" (Math|Transform|MakeTransform (Math|Vector|MakeVector _x 1.0 (+ _z 2e+01)) "0, 0, 0" "1.000000,1.000000,1.000000") "AlwaysSpawn" "MultiplyWithRoot" 0 Text 0)
  (CallFunction|SpawnHitEffect))

(event Custom|ShowCloseWidget
  (params (Widgets :type E_GameWidgets%20Enum :default "NewEnumerator0") (Show :type Boolean))
  ;[0.09466 1 0 0.5] ShowClose Widget
  (if Show
    (CallFunction|IShowWidgets Widgets)
    (else
      (CallFunction|IHideWidgets Widgets))))

(event Custom|CreateShopItemCards
  ;[0.009768 0.1251 0.15 0.5] Item
  (Utilities|Array|Clear (Variables|Default|GetShopItemCards))
  (bind _outrownames (DataTable|GetDataTableRowNames "/Game/BluePrints/DataTables/DT_ItemInfo.DT_ItemInfo"))
  (for _array_element _outrownames
    (bind _returnvalue (UserInterface|CreateWidget "/Game/UI/WB_ShopItemCard.WB_ShopItemCard_C" 0 (CallFunction|FGetItemInfo (Utilities|String|ToString(Name) _array_element))))
    (Utilities|Array|Add (Variables|Default|GetShopItemCards) _returnvalue))
  (CallFunction|DisplayShopItemCards)
  (CallFunction|IUpdateShopItemCardBuyTextColor))

(event Custom|DisplayShopItemCards
  ;[0.009768 0.1251 0.15 0.5] Item
  (Widget|Panel|ClearChildren (Variables|/Game/UI/WB_MaınUI.WB_MaınUI_C|GetVB_ItemList (Variables|Widgets|GetWB_Main)))
  (for _array_element (Variables|Default|GetShopItemCards)
    (Class|VerticalBox|AddChildtoVerticalBox (Variables|/Game/UI/WB_MaınUI.WB_MaınUI_C|GetVB_ItemList (Variables|Widgets|GetWB_Main)) _array_element)))

(event Custom|SpawnItem
  (params (Item :type Actor%20Class%20Reference) (Spawn%20Transform%20Location :type Vector))
  ;[0.009768 0.1251 0.15 0.5] Item
  (Game|SpawnActorfromClass Item (Math|Transform|MakeTransform Spawn%20Transform%20Location "0, 0, 0" "1.000000,1.000000,1.000000") "Undefined" "MultiplyWithRoot" 0 0))

(event Custom|InitializePlayer
  ;[0.1414 0.1986 0.6615 0.5] InitializePlayer
  (bind _returnvalue (UserInterface|CreateWidget "/Game/UI/WB_ShopToolTip.WB_ShopToolTip_C"))
  (Variables|Widgets|SetToolTip _returnvalue)
  (bind _returnvalue_2 (UserInterface|CreateWidget "/Game/UI/WB_MouseCursor.WB_MouseCursor_C"))
  (bind _output_get (Variables|Widgets|SetMouse%20Cursor _returnvalue_2))
  (Class|PlayerController|SetMouseCursorWidget "Default" _output_get))

(event Custom|AddLevelButtonUI
  (params (Level :type Integer))
  ;[0.05581 0.15 0.005377 0.5] Level Button UI
  (bind _returnvalue (UserInterface|CreateWidget "/Game/UI/WB_LevelCard.WB_LevelCard_C" 0 Level))
  (Class|VerticalBox|AddChildtoVerticalBox (Variables|/Game/UI/WB_MaınUI.WB_MaınUI_C|GetVB_LevelList (Variables|Widgets|GetWB_Main)) _returnvalue))

(event EventBeginPlay
  ;[0.15 0.15 0.15 0.5] Event Begin Play
  (bind _player (Class|BPIPlayer|GetPlayerRef(Message) (Game|GetPlayerCharacter 0)))
  (Variables|Default|SetPlayerPawn _player)
  (CallFunction|ShowCloseWidget "NewEnumerator0" true)
  (CallFunction|InitializePlayer)
  (CallFunction|CreateShopItemCards)
  (CallFunction|AddLevelButtonUI 1))

(fn ConstructionScript)

(fn IShowWidgets
  (params (Widget :type E_GameWidgets%20Enum :default "NewEnumerator0"))
  (switch Utilities|FlowControl|Switch|SwitchonE_GameWidgets Widget
    (:NewEnumerator0
      (Variables|Widgets|GetWB_Main
        (:then
          _)
        (:else
          (bind _returnvalue (UserInterface|CreateWidget "/Game/UI/WB_MaınUI.WB_MaınUI_C"))
          (bind _output_get (Variables|Widgets|SetWB_Main _returnvalue))))
      (UserInterface|Viewport|AddtoViewport _output_get 0))
    (:NewEnumerator2
      (Variables|Widgets|GetAscensionPopUp
        (:then
          _)
        (:else
          (bind _returnvalue_2 (UserInterface|CreateWidget "/Game/UI/WB_AscensionPopUp.WB_AscensionPopUp_C"))
          (bind _output_get_2 (Variables|Widgets|SetAscensionPopUp _returnvalue_2))))
      (UserInterface|Viewport|AddtoViewport _output_get_2 0))))

(fn IHideWidgets
  (params (Widget :type E_GameWidgets%20Enum :default "NewEnumerator0"))
  (switch Utilities|FlowControl|Switch|SwitchonE_GameWidgets Widget
    (:NewEnumerator0
      (bind _wb_main (Variables|Widgets|GetWB_Main)
        (:then
          (Widget|RemovefromParent _wb_main))
        (:else)))
    (:NewEnumerator2
      (bind _ascensionpopup (Variables|Widgets|GetAscensionPopUp)
        (:then
          (Widget|RemovefromParent _ascensionpopup))
        (:else)))))

(fn IUpdateShopItemCardBuyTextColor
  (for _array_element (Variables|Default|GetShopItemCards)
    (Appearance|SetColorandOpacity (Variables|/Game/UI/WB_ShopItemCard.WB_ShopItemCard_C|GetTXT_Buy _array_element) (Utilities|Struct|MakeSlateColor (Math|Color|SelectColor "(R=0.768628,G=0.078431,B=0.066667,A=1.000000)" "(R=0.290196,G=0.643137,B=0.094118,A=1.000000)" (> (Default|IGetItemCost (Variables|Default|GetPlayerPawn) (Variables|/Game/UI/WB_ShopItemCard.WB_ShopItemCard_C|GetItemInfo _array_element)) (Variables|/Game/BluePrints/Player/BP_Character.BP_Character_C|GetAmountOfCoins (Variables|Default|GetPlayerPawn))))) :!class /Script/UMG.TextBlock)
    (Widget|SetIsEnabled (Variables|/Game/UI/WB_ShopItemCard.WB_ShopItemCard_C|GetBTN_Buy _array_element) (select (> (Default|IGetItemCost (Variables|Default|GetPlayerPawn) (Variables|/Game/UI/WB_ShopItemCard.WB_ShopItemCard_C|GetItemInfo _array_element)) (Variables|/Game/BluePrints/Player/BP_Character.BP_Character_C|GetAmountOfCoins (Variables|Default|GetPlayerPawn))) false true))))

(fn GetPlayerControllerReferences
  (return self))