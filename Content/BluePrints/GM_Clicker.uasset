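; Game mode for a clicker game that runs level progression, enemy rounds and ascension.
; Data lookups choose each level's enemy, spawned through the player controller, and a looping timer restores its health when time runs out.
; At start it expands placed item spawn points into per-item grids of positions, served through a getter.
; Owning every shop item reveals ascension; restarting raises the ascension level and resets levels, coins, items and damage.
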(event Custom|UnlockLevel
  ;[0.15 0.05745 0.07396 0.5] Unlock Level
  (if (== (Variables|Level|GetUnlockedLevel) (Variables|Level|GetCurrentLevel))
    (bind _result (Math|Integer|IncrementInt (Variables|Level|GetUnlockedLevel))
      (:%20%20
        (if (<= _result (Variables|Level|GetMaxLevel))
          (Default|AddLevelButtonUI (Variables|References|GetPlayer%20Controller) (Variables|Level|GetUnlockedLevel))
          (Audio|PlaySound2D (select (Utilities|Enum|Equal(Enum) (.EnemyType (Utilities|Struct|BreakST_EnemyInfo (CallFunction|FGetEnemyInfo (Utilities|Struct|BreakST_LevelInfo (CallFunction|FGetLevelInfo (Variables|Level|GetUnlockedLevel)))))) "NewEnumerator0") "/Game/Audio/SC_LevelUnlocked_Normal_Cue.SC_LevelUnlocked_Normal_Cue" "/Game/Audio/SC_LevelUnlocked_Boss_Cue.SC_LevelUnlocked_Boss_Cue") 1.0 1.0 0.0 0 0))))))

(event Custom|SetCurrentLevel
  (params (Level :type Integer))
  (bind (_enemy _spawntransform) (CallFunction|GetEnemytoSpawnforCurrentLevel))
  ;[0 0.774 0.4627 0.5] SetCurrentLevel
  (Variables|Level|SetCurrentLevel Level)
  (bind _spawnedenemy (Variables|/Game/BluePrints/PC_Clicker.PC_Clicker_C|GetSpawnedEnemy (Variables|References|GetPlayer%20Controller))
    (:then
      (Actor|DestroyActor _spawnedenemy))
    (:else
      _))
  (Default|SpawnEnemy (Variables|References|GetPlayer%20Controller) _enemy _spawntransform)
  (CallFunction|StartRoundTimer))

(event Custom|StartRoundTimer
  ;[0.15 0.134 0.02343 0.5] RoundTimerLoop
  (Variables|Timer|SetCurrentRoundTimer (Variables|Timer|GetInıtialRoundTimer))
  (bind _returnvalue (Utilities|Time|SetTimerbyEvent (delegate Custom|RoundTimerLoop) (Variables|Timer|GetRoundTimerTime) true))
  (Variables|Default|SetRoundTimerHandle _returnvalue))

(event Custom|RoundTimerLoop
  ;[0.15 0.134 0.02343 0.5] RoundTimerLoop
  (bind _output_get (Variables|Timer|SetCurrentRoundTimer (Math|Float|Clamp(Float) (- (Variables|Timer|GetCurrentRoundTimer) (Variables|Timer|GetRoundTimerTime)) 0.0 (Variables|Timer|GetCurrentRoundTimer))))
  (Default|UpdateTimerUI (Variables|/Game/BluePrints/PC_Clicker.PC_Clicker_C|GetWB_Main (Variables|References|GetPlayer%20Controller)) _output_get)
  (if (== (Variables|Timer|GetCurrentRoundTimer) 0.0)
    (Default|RestoreGealth (Variables|/Game/BluePrints/PC_Clicker.PC_Clicker_C|GetSpawnedEnemy (Variables|References|GetPlayer%20Controller)))
    (Variables|Timer|SetCurrentRoundTimer (Variables|Timer|GetInıtialRoundTimer))))

(event Custom|RestartGame
  (bind _player_controller (Variables|References|GetPlayer%20Controller))
  (bind _playerpawn (Variables|References|GetPlayerPawn))
  ;[0.1227 0.15 0 0.5] RestartGame
  (Math|Integer|IncrementInt (Variables|Ascension|GetAscensionLevel)
    (:%20%20
      (Variables|Ascension|SetAscensionCriteriaMet? false)
      (Variables|Level|SetUnlockedLevel 1)
      (Variables|Level|SetCurrentLevel 1)
      (Widget|Panel|ClearChildren (Variables|/Game/UI/WB_MaınUI.WB_MaınUI_C|GetVB_LevelList (Variables|/Game/BluePrints/PC_Clicker.PC_Clicker_C|GetWB_Main _player_controller)))
      (Default|AddLevelButtonUI _player_controller (Variables|Level|GetUnlockedLevel))
      (bind _output_get (Variables|/Game/BluePrints/Player/BP_Character.BP_Character_C|SetAmountOfCoins (Variables|References|GetPlayerPawn) 0))
      (Default|UpdateCoinsAmountUI (Variables|/Game/BluePrints/PC_Clicker.PC_Clicker_C|GetWB_Main (Variables|References|GetPlayer%20Controller)) _output_get)
      (Utilities|Map|Clear (Variables|/Game/BluePrints/Player/BP_Character.BP_Character_C|GetItemsBought (Variables|References|GetPlayerPawn)))
      (Default|CreateShopItemCards (Variables|References|GetPlayer%20Controller))
      (Variables|/Game/BluePrints/Player/BP_Character.BP_Character_C|SetTotalDPS _playerpawn 0.0)
      (Variables|/Game/BluePrints/Player/BP_Character.BP_Character_C|SetCursorDamage _playerpawn 15.0)
      (CallFunction|SetCurrentLevel (Variables|Level|GetCurrentLevel))
      (Utilities|Map|Clear (Variables|/Game/BluePrints/Player/BP_Character.BP_Character_C|GetItemsBought (Variables|References|GetPlayerPawn))))))

(event EventBeginPlay
  (bind (_enemy _spawntransform) (CallFunction|GetEnemytoSpawnforCurrentLevel))
  ;[0.143 0.0576 0.15 0.5] Event Begin Play
  (bind _returnvalue (Actor|GetActorOfClass "/Game/BluePrints/SpawnPoints/BP_Enemy_SpawnPint.BP_Enemy_SpawnPint_C"))
  (Variables|Default|SetEnemySpawn _returnvalue)
  (bind _playercontroller (Class|BPIPlayerController|GetPlayerControllerReferences(Message) (Game|GetPlayerController 0)))
  (bind _output_get (Variables|References|SetPlayer%20Controller _playercontroller))
  (bind _player (Class|BPIPlayer|GetPlayerRef(Message) (Game|GetPlayerCharacter 0)))
  (Variables|References|SetPlayerPawn _player)
  (CallFunction|SetItemSpawmPoints)
  (bind _outrownames (DataTable|GetDataTableRowNames "/Game/BluePrints/DataTables/DT_ItemInfo.DT_ItemInfo"))
  (Variables|Default|SetAmountOfShopItems (Utilities|Array|Length _outrownames))
  (Default|SpawnEnemy _output_get _enemy _spawntransform)
  (CallFunction|StartRoundTimer))

(fn ConstructionScript)

(fn GetEnemytoSpawnforCurrentLevel
  (return (Utilities|Struct|BreakST_EnemyInfo (CallFunction|FGetEnemyInfo (Utilities|Struct|BreakST_LevelInfo (CallFunction|FGetLevelInfo (Variables|Level|GetCurrentLevel))))) (Transformation|GetActorTransform (Variables|Default|GetEnemySpawn))))

(fn SetItemSpawmPoints
  (bind _outactors (Actor|GetAllActorsOfClass "/Game/BluePrints/SpawnPoints/BP_ItemSpawnPoint.BP_ItemSpawnPoint_C"))
  (bind _output_get (LocalVariables|SetLocalItemSpawnPoint _outactors))
  (if (> (Utilities|Array|Length _output_get) 0)
    (for _index (range 0 (LocalVariables|GetLocalLoopLastIndex)) :!label _label
      (Utilities|Array|Add (Utilities|Select :Index (Variables|/Game/BluePrints/SpawnPoints/BP_ItemSpawnPoint.BP_ItemSpawnPoint_C|GetItem (Utilities|Array|Get(acopy) (LocalVariables|GetLocalItemSpawnPoint))) :NewEnumerator1 (Variables|ItemSpawnPoints|GetCursorSpawnPoint) :NewEnumerator0 (Variables|ItemSpawnPoints|GetTorchSpawnPoints) :NewEnumerator2 (Variables|ItemSpawnPoints|GetGrandWizardHatSpawnPoint) :NewEnumerator3 (Variables|ItemSpawnPoints|GetKingsCrownSpawnPoint) :NewEnumerator4 (Variables|ItemSpawnPoints|GetKnightHelmetSpawnPoint) :NewEnumerator5 (Variables|ItemSpawnPoints|GetLightFeatherSpawnPoint) :NewEnumerator6 (Variables|ItemSpawnPoints|GetLuckyRainbowSpawnPoint) :NewEnumerator7 (Variables|ItemSpawnPoints|GetOrcSkullSpawnPoint) :NewEnumerator8 (Variables|ItemSpawnPoints|GetRuneOfTimeSpawnPoint) :NewEnumerator9 (Variables|ItemSpawnPoints|GetTheProtectorSpawnPoint) :NewEnumerator10 (Variables|ItemSpawnPoints|GetCrownOfEvilSpawnPoint)) (Math|Vector|MakeVector (+ (.x (Transformation|GetActorLocation (Utilities|Array|Get(acopy) (LocalVariables|GetLocalItemSpawnPoint)))) (* 9.0 _index)) (.y (Transformation|GetActorLocation (Utilities|Array|Get(acopy) (LocalVariables|GetLocalItemSpawnPoint)))) (- (.z (Transformation|GetActorLocation (Utilities|Array|Get(acopy) (LocalVariables|GetLocalItemSpawnPoint)))) (* 13 (LocalVariables|GetLocalZAxisMultiplayer)))))
      (if (== (LocalVariables|GetLocalLoopLastIndex) _index)
        (bind _result (Math|Integer|IncrementInt (LocalVariables|GetLocalLoopCounter))
          (:%20%20
            (if (< _result (LocalVariables|GetLocalAmountOfRows))
              (Math|Integer|IncrementInt (LocalVariables|GetLocalZAxisMultiplayer)
                (:%20%20
                  (goto _label)))
              (else
                (Utilities|Array|RemoveIndex (LocalVariables|GetLocalItemSpawnPoint))
                (if (Utilities|Array|IsNotEmpty (LocalVariables|GetLocalItemSpawnPoint))
                  (LocalVariables|SetLocalZAxisMultiplayer 0)
                  (LocalVariables|SetLocalLoopCounter 0)
                  (goto _label))))))))))

(fn IGetItemSpawnPoints
  (params (Item%20Name :type E_Items%20Enum :default "NewEnumerator0"))
  (switch Utilities|FlowControl|Switch|SwitchonE_Items Item%20Name
    (:NewEnumerator1
      (return (Variables|ItemSpawnPoints|GetCursorSpawnPoint)))
    (:NewEnumerator0
      (return (Variables|ItemSpawnPoints|GetTorchSpawnPoints)))
    (:NewEnumerator2
      (return (Variables|ItemSpawnPoints|GetGrandWizardHatSpawnPoint)))
    (:NewEnumerator3
      (return (Variables|ItemSpawnPoints|GetKingsCrownSpawnPoint)))
    (:NewEnumerator4
      (return (Variables|ItemSpawnPoints|GetKnightHelmetSpawnPoint)))
    (:NewEnumerator5
      (return (Variables|ItemSpawnPoints|GetLightFeatherSpawnPoint)))
    (:NewEnumerator6
      (return (Variables|ItemSpawnPoints|GetLuckyRainbowSpawnPoint)))
    (:NewEnumerator7
      (return (Variables|ItemSpawnPoints|GetOrcSkullSpawnPoint)))
    (:NewEnumerator8
      (return (Variables|ItemSpawnPoints|GetRuneOfTimeSpawnPoint)))
    (:NewEnumerator9
      (return (Variables|ItemSpawnPoints|GetTheProtectorSpawnPoint)))
    (:NewEnumerator10
      (return (Variables|ItemSpawnPoints|GetCrownOfEvilSpawnPoint)))))

(fn ICheckAscensionCriteriaMet
  (if (not (Variables|Ascension|GetAscensionCriteriaMet?))
    (bind _keys (Utilities|Map|Keys (Variables|/Game/BluePrints/Player/BP_Character.BP_Character_C|GetItemsBought (Variables|References|GetPlayerPawn))))
    (if (== (Utilities|Array|Length _keys) (Variables|Default|GetAmountOfShopItems))
      (bind _values (Utilities|Map|Values (Variables|/Game/BluePrints/Player/BP_Character.BP_Character_C|GetItemsBought (Variables|References|GetPlayerPawn))))
      (bind _array_element (Utilities|Array|ForEachLoopwithBreak _values :!label _label)
        (:LoopBody
          (if (>= _array_element 1)
            (Math|Integer|IncrementInt (LocalVariables|GetLocalCounter))
            (else
              (goto _label Break))))
        (:Completed
          (if (== (LocalVariables|GetLocalCounter) (Variables|Default|GetAmountOfShopItems))
            (Variables|Ascension|SetAscensionCriteriaMet? true)
            (Widget|SetVisibility (Variables|/Game/UI/WB_MaınUI.WB_MaınUI_C|GetOV_Ascension (Variables|/Game/BluePrints/PC_Clicker.PC_Clicker_C|GetWB_Main (Variables|References|GetPlayer%20Controller))) "SelfHitTestInvisible")))))))

(fn GetGameModeReferences
  (return self))