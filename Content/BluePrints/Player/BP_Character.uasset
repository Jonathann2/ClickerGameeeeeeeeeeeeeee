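; Player character for a clicker game that holds the coin balance, bought item counts, cursor damage and total DPS.
; Purchases deduct coins, refresh shop UI, spawn the item, update cursor damage or passive DPS with the ascension multiplier, and trigger the GameMode's ascension check.
; A looping timer applies DPS, scaled to its interval, to the spawned enemy.
; Enhanced Input clicks swap the mouse cursor image.
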(event Custom|UpdateAmountOfCoins
  (params (AmountOfCoins :type Integer) (bAdd :type Boolean))
  ;[0.15 0.1423 0.03932 0.5] UpdateCoin
  (bind _output_get (Variables|Default|SetAmountOfCoins (select bAdd (+ AmountOfCoins (Variables|Default|GetAmountOfCoins)) (- AmountOfCoins (Variables|Default|GetAmountOfCoins)))))
  (Default|UpdateCoinsAmountUI (Variables|/Game/BluePrints/PC_Clicker.PC_Clicker_C|GetWB_Main (Variables|Default|GetPlayer%20Controller)) _output_get))

(event Custom|UpdateAmountOfGoldByHit
  (params (GoldByHit :type Integer) (Add :type Boolean))
  ;[0.15 0.1428 0.031 0.5] Gold By Hit
  (bind _output_get (Variables|Default|SetAmountOfCoins (select Add (+ GoldByHit (Variables|Default|GetAmountOfCoins)) (- GoldByHit (Variables|Default|GetAmountOfCoins)))))
  (Default|UpdateCoinsAmountUI (Variables|/Game/BluePrints/PC_Clicker.PC_Clicker_C|GetWB_Main (Variables|Default|GetPlayer%20Controller)) _output_get))

(event Custom|PurchaseItem
  (params (Item :type ST%20Item%20Info%20Structure) (ShopItemCard :type WB%20Shop%20Item%20Card%20Object%20Reference))
  (bind (_name _item _dps) (Utilities|Struct|BreakST_ItemInfo Item))
  (bind _player_controller (Variables|Default|GetPlayer%20Controller))
  (bind _itemsbought (Variables|Default|GetItemsBought))
  (bind _value (Utilities|Map|Find _itemsbought _name))
  ;[0.15 0.15 0.15 0.5] PurchaseItem
  (Audio|PlaySound2D "/Game/Audio/SC_Purchase_Cue.SC_Purchase_Cue" 1.0 1.0 0.0 0 0)
  (bind _output_get (Variables|Default|SetAmountOfCoins (- (Variables|Default|GetAmountOfCoins) (CallFunction|IGetItemCost Item))))
  (Default|UpdateCoinsAmountUI (Variables|/Game/BluePrints/PC_Clicker.PC_Clicker_C|GetWB_Main (Variables|Default|GetPlayer%20Controller)) _output_get)
  (Utilities|Map|Add (Variables|Default|GetItemsBought) _name (+ _value 1))
  (Default|UpdateItemsBoughtUI ShopItemCard)
  (Default|UpdateItemCost ShopItemCard)
  (Default|IUpdateShopItemCardBuyTextColor _player_controller)
  (Default|SpawnItem _player_controller (.CLass (Utilities|Struct|BreakST_ItemInfo Item)) (Utilities|Array|Get(acopy) (Default|IGetItemSpawnPoints (Variables|Default|GetGame%20Mode) _item) (- _value 1)))
  (if (Utilities|Enum|Equal(Enum) _item "NewEnumerator1")
    (CallFunction|IIncreaseCursorDamage (* _dps (Utilities|Struct|BreakST_Ascension (CallFunction|FGetAscensionMlt (Variables|/Game/BluePrints/GM_Clicker.GM_Clicker_C|GetAscensionLevel (Variables|Default|GetGame%20Mode))))))
    (else
      (CallFunction|IUpdateTotalDPS)))
  (Default|UpdateToolTipUI (Variables|/Game/BluePrints/PC_Clicker.PC_Clicker_C|GetToolTip (Variables|Default|GetPlayer%20Controller)) Item)
  (Default|ICheckAscensionCriteriaMet (Variables|Default|GetGame%20Mode)))

(event Custom|AutoDamageLoop
  ;[0.15 0.15 0.15 0.5] Auto Damage Loop
  (bind _returnvalue (Utilities|Time|SetTimerbyFunctionName 0 "I_AutoDamage" (Variables|Damage|GetAutoDamageTimerTime) true))
  (Variables|Damage|SetAutoDamageHandle _returnvalue))

(event Input|EnhancedActionEvents|EnhancedInputActionM_MouseClickCursor
  (params (ActionValue :type Boolean) (ElapsedSeconds :type Float%20%28double-precision%29) (TriggeredSeconds :type Float%20%28double-precision%29) (InputAction :type Input%20Action%20Object%20Reference :default "/Game/BluePrints/Player/Inputs/M_MouseClickCursor.M_MouseClickCursor"))
  (bind _player_controller (Variables|Default|GetPlayer%20Controller))
  (bind _mouse_cursor (Variables|/Game/BluePrints/PC_Clicker.PC_Clicker_C|GetMouse%20Cursor _player_controller))
  ;[0.15 0.15 0.15 0.5] InputAction
  (:Triggered
    (Default|SetMouseCursorImage _mouse_cursor "NewEnumerator1"))
  (:Completed
    (Default|SetMouseCursorImage _mouse_cursor "NewEnumerator0")))

(event EventBeginPlay
  ;[0.15 0.15 0.15 0.5] Event Begin Play
  (bind _playercontroller (Class|BPIPlayerController|GetPlayerControllerReferences(Message) (Game|GetPlayerController 0)))
  (Variables|Default|SetPlayer%20Controller _playercontroller)
  (bind _gamemode (Class|BPIGameMode|GetGameModeReferences(Message) (Game|GetGameMode)))
  (Variables|Default|SetGame%20Mode _gamemode)
  (Utilities|IsValid (PlayerController|LocalPlayerSubsystems|GetEnhancedInputLocalPlayerSubsystem (Variables|Default|GetPlayer%20Controller))
    (:Is%20Valid
      (Input|AddMappingContext (PlayerController|LocalPlayerSubsystems|GetEnhancedInputLocalPlayerSubsystem (Variables|Default|GetPlayer%20Controller)) "/Game/BluePrints/Player/Inputs/IMC_Default.IMC_Default" 0 "(bIgnoreAllPressedKeysUntilRelease=True,bForceImmediately=False,bNotifyUserSettings=False)")
      (Default|UpdateCoinsAmountUI (Variables|/Game/BluePrints/PC_Clicker.PC_Clicker_C|GetWB_Main (Variables|Default|GetPlayer%20Controller)) (Variables|Default|GetAmountOfCoins))
      (CallFunction|AutoDamageLoop))))

(fn ConstructionScript)

(fn IDoesPlayerHasEnoughCoins
  (params (ItemCost :type Integer))
  (return (>= (Variables|Default|GetAmountOfCoins) ItemCost)))

(fn IGetItemCost
  (params (Item :type ST%20Item%20Info%20Structure))
  (bind (_name _item) (Utilities|Struct|BreakST_ItemInfo Item))
  (bind _itemsbought (Variables|Default|GetItemsBought))
  (bind _value (Utilities|Map|Find _itemsbought _name))
  (bind _item_cost (CallFunction|FGetItemCost _value))
  (bind (_torch _cursor _grandwizardhat _kingscrown _knighthelmet _lightfeather _luckyrainbow _orcskull _runeoftime _theprotector _crownofevil) (Utilities|Struct|BreakST_ItemCost _item_cost))
  (return (Utilities|Select :Index _item :NewEnumerator1 _cursor :NewEnumerator0 _torch :NewEnumerator2 _grandwizardhat :NewEnumerator3 _kingscrown :NewEnumerator4 _knighthelmet :NewEnumerator5 _lightfeather :NewEnumerator6 _luckyrainbow :NewEnumerator7 _orcskull :NewEnumerator8 _runeoftime :NewEnumerator9 _theprotector :NewEnumerator10 _crownofevil)))

(fn IAutoDamage
  (Game|Damage|ApplyDamage (Variables|/Game/BluePrints/PC_Clicker.PC_Clicker_C|GetSpawnedEnemy (Variables|Default|GetPlayer%20Controller)) (/ (Variables|Damage|GetTotalDPS) (/ 1.0 (Variables|Damage|GetAutoDamageTimerTime))) 0 0 "/Game/BluePrints/BP_AutoDamage.BP_AutoDamage_C"))

(fn IUpdateTotalDPS
  (bind _keys (Utilities|Map|Keys (Variables|Default|GetItemsBought)))
  (for (_array_element _array_index) _keys
    (if (Utilities|Enum|NotEqual(Enum) (.Item (Utilities|Struct|BreakST_ItemInfo (CallFunction|FGetItemInfo _array_element))) "NewEnumerator1")
      (bind _values (Utilities|Map|Values (Variables|Default|GetItemsBought)))
      (LocalVariables|SetLocalTotalDPS (+ (LocalVariables|GetLocalTotalDPS) (* (Utilities|Array|Get(acopy) _values _array_index) (* (.DPS (Utilities|Struct|BreakST_ItemInfo (CallFunction|FGetItemInfo _array_element))) (Utilities|Struct|BreakST_Ascension (CallFunction|FGetAscensionMlt (Variables|/Game/BluePrints/GM_Clicker.GM_Clicker_C|GetAscensionLevel (Variables|Default|GetGame%20Mode))))))))))
  (Variables|Damage|SetTotalDPS (LocalVariables|GetLocalTotalDPS)))

(fn IIncreaseCursorDamage
  (params (DamageToAdd :type Float%20%28double-precision%29))
  (Variables|Damage|SetCursorDamage (+ DamageToAdd (Variables|Damage|GetCursorDamage))))

(fn GetPlayerRef
  (return self))